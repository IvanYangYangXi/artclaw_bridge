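; Spline placement tool actor that lays copies of a mesh along its spline in the Construction Script.
; It splits the spline length into SegmentCount equal segments and adds one movable component per segment.
; With CanBend on, SplineMeshComponents deform the mesh between segment endpoints using spline tangents.
; With it off, rigid StaticMeshComponents sit at each segment start, rotated toward the next point.
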(event EventBeginPlay)

(event Collision|EventActorBeginOverlap
  (params (OtherActor :type Actor%20Object%20Reference)))

(event EventTick
  (params (DeltaSeconds :type Float%20%28single-precision%29)))

(fn ConstructionScript
  (bind _returnvalue (Math|Transform|MakeTransform "0, 0, 0"))
  (bind _spline (Variables|Default|GetSpline))
  (bind _mesh (Variables|Default|GetMesh))
  (bind _spline_2 (Variables|Default|GetSpline))
  (bind _segmentcount (Variables|Default|GetSegmentCount))
  (bind _bcanbend (Variables|Default|GetbCanBend))
  (bind _returnvalue_2 (Spline|GetSplineLength _spline))
  (bind _returnvalue_3 (Math|Conversions|ToFloat(Integer) _segmentcount))
  (bind _returnvalue_4 (Math|Conversions|ToFloat(Boolean) _bcanbend))
  (for _index (range 0 (- (Variables|Default|GetSegmentCount) 1))
    (if _bcanbend
      (bind _returnvalue_5 (Game|AddComponentbyClass "/Script/Engine.SplineMeshComponent" false _returnvalue))
      (bind _as样条网格体组件 (Utilities|Casting|CastToSplineMeshComponent _returnvalue_5))
      (Components|StaticMesh|SetStaticMesh _as样条网格体组件 _mesh)
      (Transformation|SetMobility _as样条网格体组件 "Movable")
      (SplineMesh|SetStartandEnd _as样条网格体组件 (Spline|GetLocationatDistanceAlongSpline _spline_2 (* (/ (Math|Conversions|ToFloat(Integer) _index) _returnvalue_3) _returnvalue_2) "Local") (Math|Vector|Lerp(Vector) (- (Spline|GetLocationatDistanceAlongSpline _spline_2 (* (/ (Math|Conversions|ToFloat(Integer) (+ _index 1)) _returnvalue_3) _returnvalue_2) "Local") (Spline|GetLocationatDistanceAlongSpline _spline_2 (* (/ (Math|Conversions|ToFloat(Integer) _index) _returnvalue_3) _returnvalue_2) "Local")) (Spline|GetTangentatDistanceAlongSpline _spline_2 (* (/ (Math|Conversions|ToFloat(Integer) _index) _returnvalue_3) _returnvalue_2) "Local") _returnvalue_4) (Spline|GetLocationatDistanceAlongSpline _spline_2 (* (/ (Math|Conversions|ToFloat(Integer) (+ _index 1)) _returnvalue_3) _returnvalue_2) "Local") (Math|Vector|Lerp(Vector) (- (Spline|GetLocationatDistanceAlongSpline _spline_2 (* (/ (Math|Conversions|ToFloat(Integer) (+ _index 1)) _returnvalue_3) _returnvalue_2) "Local") (Spline|GetLocationatDistanceAlongSpline _spline_2 (* (/ (Math|Conversions|ToFloat(Integer) _index) _returnvalue_3) _returnvalue_2) "Local")) (Spline|GetTangentatDistanceAlongSpline _spline_2 (* (/ (Math|Conversions|ToFloat(Integer) (+ _index 1)) _returnvalue_3) _returnvalue_2) "Local") _returnvalue_4) true :!class /Script/Engine.SplineMeshComponent)
      (else
        (bind _returnvalue_6 (Game|AddComponentbyClass "/Script/Engine.StaticMeshComponent" false _returnvalue))
        (bind _as静态网格体组件 (Utilities|Casting|CastToStaticMeshComponent _returnvalue_6))
        (Components|StaticMesh|SetStaticMesh _as静态网格体组件 _mesh)
        (Transformation|SetMobility _as静态网格体组件 "Movable")
        (Transformation|SetRelativeLocation _as静态网格体组件 (Spline|GetLocationatDistanceAlongSpline _spline_2 (* (/ (Math|Conversions|ToFloat(Integer) _index) _returnvalue_3) _returnvalue_2) "Local") false false)
        (Transformation|SetRelativeRotation _as静态网格体组件 (Math|Rotator|MakeRotfromX (Math|Vector|Normalize (- (Spline|GetLocationatDistanceAlongSpline _spline_2 (* (/ (Math|Conversions|ToFloat(Integer) (+ _index 1)) _returnvalue_3) _returnvalue_2) "Local") (Spline|GetLocationatDistanceAlongSpline _spline_2 (* (/ (Math|Conversions|ToFloat(Integer) _index) _returnvalue_3) _returnvalue_2) "Local")))) false false)))))